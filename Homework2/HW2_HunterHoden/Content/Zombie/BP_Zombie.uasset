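; Zombie enemy for a VR game that chases the player with AIMoveTo, loops an attack montage on arrival and speeds adjust on sighting through PawnSensing.
; Its Sphere overlap damages whatever enters it; a radius-based hit check is left unwired.
; Projectile overlaps on the capsule lower Health, and a hit at zero destroys it and calls ZombiesKilled on VRPawn.
; The montage-based Death event is not called here.
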(event `self.ReceiveBeginPlay`
  (`self.Run To Player`)
  (set `self.Health` 100))

(event `Run To Player`
  (`|AIMoveTo` self (0.0 0.0 0.0) (`GameplayStatics.GetPlayerController` 0) 40.0
    (:`OnSuccess`
      (`self.Attack Player`))
    (:`OnFail`
      (`self.Run To Player`))))

(event `self.PawnSensing.OnSeePawn`
  (params (Pawn :type "Pawn Object Reference"))
  (set `CharacterMovementComponent.MaxWalkSpeed` 360.0 (`self.CharacterMovement`)))

(event `Attack Player`
  (`|PlayMontage` (`self.Mesh`) "/Game/Zombie/Animation/zombie_attack_Montage1.zombie_attack_Montage1"
    (:`OnCompleted`
      (`self.Run To Player`))))

(event `self.CapsuleComponent.OnComponentBeginOverlap`
  (params (OverlappedComponent :type "PrimitiveComponent Object Reference") (OtherActor :type "Actor Object Reference") (OtherComp :type "PrimitiveComponent Object Reference") (OtherBodyIndex :type Integer) (bFromSweep :type Boolean) (SweepResult :type "HitResult Structure (by ref)"))
  (if (== (`GameplayStatics.GetObjectClass` OtherActor) "/Game/VRTemplate/Blueprints/Projectile.Projectile_C")
    (`self.Health_Decrease`)))

(event `Death`
  (`|PlayMontage` (`self.Mesh`)
    (:`OnCompleted`
      (`self.K2_DestroyActor`))))

(event `self.Sphere.OnComponentBeginOverlap`
  (params (OverlappedComponent :type "PrimitiveComponent Object Reference") (OtherActor :type "Actor Object Reference") (OtherComp :type "PrimitiveComponent Object Reference") (OtherBodyIndex :type Integer) (bFromSweep :type Boolean) (SweepResult :type "HitResult Structure (by ref)"))
  (`GameplayStatics.ApplyDamage` OtherActor 20.0))

(fn `Health_Decrease`
  (if (> (`self.Health`) 0)
    (set `self.Health` (- (`self.Health`) 20))
    (else
      (`self.K2_DestroyActor`)
      (bind _returnvalue (`GameplayStatics.GetActorOfClass` "/Game/VRTemplate/Blueprints/VRPawn.VRPawn_C"))
      (`/Game/VRTemplate/Blueprints/VRPawn.ZombiesKilled` _returnvalue))))

(fn `UserConstructionScript`)